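; Pistol weapon Blueprint that fires first-person projectiles, limited by magazine count and a fire cooldown.
; WeaponFire checks the cooldown flag and Mag, calls Fire, decrements the clamped count, has the player check ammo, then re-enables firing after a delay.
; Fire spawns BP_FirstPersonProjectile at the gun's Ammo socket plus a camera-rotated offset, oriented along the camera rotation.
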(event `/Game/Blueprints/Weapon_BPs/BPI_WeaponFire.WeaponFire`
  (bind _player_ref (`self.Player ref`))
  (if (`self.FireTimeFinished`)
    (if (!= (`self.mag`) 0)
      (`/Game/Blueprints/Weapon_BPs/Weapon_Pickups/BPI_Fire.Fire`)
      (set `self.mag` (`KismetMathLibrary.Clamp` (- (`self.mag`) 1) 0 (`self.mag size`)))
      (set `self.FireTimeFinished` false)
      (`/Game/FirstPerson/Blueprints/BP_FirstPersonCharacter.CheckAmmo` _player_ref (`/Game/FirstPerson/Blueprints/BP_FirstPersonCharacter.CurrentWeapon` _player_ref))
      (`KismetSystemLibrary.Delay` 1.0)
      (set `self.FireTimeFinished` true)
      (`KismetSystemLibrary.PrintString` "Delay done")
      (else
        (`KismetSystemLibrary.PrintString` "NO BULLETS")))))

(event `/Game/Blueprints/Weapon_BPs/Weapon_Pickups/BPI_Fire.Fire`
  (bind _returnvalue (`PlayerCameraManager.GetCameraRotation` (`GameplayStatics.GetPlayerCameraManager` 0)))
  (`|SpawnActorFromClass` "/Game/FirstPerson/Blueprints/BP_FirstPersonProjectile.BP_FirstPersonProjectile_C" (`KismetMathLibrary.MakeTransform` (+ (`SceneComponent.GetSocketLocation` (`self.GunMesh`) "Ammo") (`KismetMathLibrary.GreaterGreater_VectorRotator` (`self.Projectile Offset`) _returnvalue)) _returnvalue) "Undefined" "OverrideRootScale" null null))

(fn `UserConstructionScript`
  (`parent.UserConstructionScript`))