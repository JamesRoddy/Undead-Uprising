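; Zombie AI character that takes bullet damage and dies in the game.
; Capsule overlaps fire a Niagara effect while alive; components tagged "Bullet" reduce health and are destroyed, and a lethal hit plays a one-shot falling death animation.
; Tick halts AI movement and logic at zero health, then destroys the actor after a delay.
; While alive, Tick uses a dot product to tell the anim blueprint whether the player is in front.
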(event `self.ReceiveTick`
  (params (DeltaSeconds :type "Float (single-precision)"))
  (bind _returnvalue (`AIBlueprintHelperLibrary.GetAIController` (`self.ControlledPawn`)))
  (if (<= (`self.zombHealth`) 0.0)
    (`Controller.StopMovement` _returnvalue)
    (`BrainComponent.StopLogic` (`AIController.BrainComponent` _returnvalue) "Death")
    (`KismetSystemLibrary.Delay` 2.5)
    (`self.K2_DestroyActor`)
    (else
      (bind _asabp_charatcer (cast `/Game/Characters/Zombie/Animations/DefaultZombieAnimations/ABP_Charatcer` (`SkeletalMeshComponent.GetAnimInstance` (`self.Mesh`)))
        (:`then`
          (if (>= (`KismetMathLibrary.Dot_VectorVector` (`self.GetActorForwardVector`) (`KismetMathLibrary.Normal` (- (`self.K2_GetActorLocation` (`GameplayStatics.GetPlayerPawn` 0)) (`self.K2_GetActorLocation`)))) 0.0)
            (set `/Game/Characters/Zombie/Animations/DefaultZombieAnimations/ABP_Charatcer.FrontTest` true _asabp_charatcer)
            (else
              (set `/Game/Characters/Zombie/Animations/DefaultZombieAnimations/ABP_Charatcer.FrontTest` false _asabp_charatcer))))
        (:`CastFailed`
          (`KismetSystemLibrary.PrintString` "Cast Failed"))))))

(event `self.CapsuleComponent.OnComponentBeginOverlap`
  (params (OverlappedComponent :type "PrimitiveComponent Object Reference") (OtherActor :type "Actor Object Reference") (OtherComp :type "PrimitiveComponent Object Reference") (OtherBodyIndex :type Integer) (bFromSweep :type Boolean) (SweepResult :type "HitResult Structure (by ref)"))
  (if (not (`self.PlayedAnim`))
    (`ActorComponent.Activate` (`self.Niagara`) true))
  (if (`ActorComponent.ComponentHasTag` OtherComp "Bullet")
    (bind _output_get (set `self.zombHealth` (- (`self.zombHealth`) 30.0)))
    (if (<= _output_get 0.0)
      (`self.K2_DestroyActor` OtherActor)
      (if (not (`self.PlayedAnim`))
        (`SkeletalMeshComponent.PlayAnimation` (`self.Mesh`) "/Game/Characters/Zombie/Animations/DefaultZombieAnimations/Falling_Back_Death.Falling_Back_Death" false)
        (set `self.PlayedAnim` true))
      (else
        (`self.K2_DestroyActor` OtherActor)))
    (else
      (`KismetSystemLibrary.PrintString` "No tag"))))

(event `self.ReceiveActorBeginOverlap`
  (params (OtherActor :type "Actor Object Reference")))

(event `self.ReceiveBeginPlay`)

(fn `UserConstructionScript`)