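; Female zombie enemy that damages the player, takes projectile hits and awards points on hit and kill.
; Tick applies damage and attack sound when the anim Blueprint's damage flag is set, and uses a dot product to tell it whether the player is in front.
; Capsule overlaps with bullet-tagged projectiles reduce health and trigger Niagara effects.
; At zero health it plays death sound and animation, then Tick stops movement, disables collision and destroys it after a delay.
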(event `self.ReceiveTick`
  (params (DeltaSeconds :type "Float (single-precision)"))
  (bind _animationref (`self.AnimationRef`))
  (`self.FemDamagingPlayer`)
  (if (<= (`self.EnemyHealth`) 0.0)
    (`Controller.StopMovement` (`self.GetController`))
    (`self.SetActorEnableCollision` false)
    (`KismetSystemLibrary.Delay` 2.5)
    (`self.K2_DestroyActor`)
    (elif (>= (`KismetMathLibrary.Dot_VectorVector` (`self.GetActorForwardVector`) (`KismetMathLibrary.Normal` (- (`self.K2_GetActorLocation` (`GameplayStatics.GetPlayerPawn` 0)) (`self.K2_GetActorLocation`)))) 0.0)
      (set `/Game/Characters/Zombie/Animations/FemZombieAnimations/ABP_FemZombie.FemFrontTest` true _animationref)
      (`KismetSystemLibrary.Delay` 1.5)
      (else
        (set `/Game/Characters/Zombie/Animations/FemZombieAnimations/ABP_FemZombie.FemFrontTest` false _animationref)
        (`KismetSystemLibrary.Delay` 1.5)))))

(event `self.CapsuleComponent.OnComponentBeginOverlap`
  (params (OverlappedComponent :type "PrimitiveComponent Object Reference") (OtherActor :type "Actor Object Reference") (OtherComp :type "PrimitiveComponent Object Reference") (OtherBodyIndex :type Integer) (bFromSweep :type Boolean) (SweepResult :type "HitResult Structure (by ref)"))
  (bind _asbp_projectile (cast `/Game/Blueprints/Weapon_BPs/BP_Projectile` OtherActor))
  (`/Game/FirstPerson/Blueprints/BP_FirstPersonCharacter.IncreasePoints` (`self.PlayerRef`) 50)
  (if (not (`self.FemPlayedAnim`))
    (`ActorComponent.Activate` (`self.Niagara`) true))
  (if (`ActorComponent.ComponentHasTag` OtherComp "Bullet")
    (bind _output_get (set `self.EnemyHealth` (- (`self.EnemyHealth`) (`/Game/Blueprints/Weapon_BPs/BP_Projectile.damage` _asbp_projectile))))
    (if (<= _output_get 0.0)
      (`/Game/FirstPerson/Blueprints/BP_FirstPersonCharacter.IncreasePoints` (`self.PlayerRef`) 150)
      (`self.K2_DestroyActor` _asbp_projectile)
      (if (not (`self.FemPlayedAnim`))
        (`AudioComponent.Play` (`self.AltDeath`) 0.0)
        (`SkeletalMeshComponent.PlayAnimation` (`self.Mesh`) "/Game/Characters/Zombie/Animations/FemZombieAnimations/FemZombieDeath.FemZombieDeath" false)
        (set `self.FemPlayedAnim` true))
      (else
        (`self.K2_DestroyActor` _asbp_projectile)))
    (else
      (`KismetSystemLibrary.PrintString` "No tag"))))

(event `self.ReceiveBeginPlay`
  (bind _returnvalue (`GameplayStatics.GetActorOfClass` "/Game/FirstPerson/Blueprints/BP_FirstPersonCharacter.BP_FirstPersonCharacter_C"))
  (set `self.PlayerRef` _returnvalue))

(fn `FemDamagingPlayer`
  (`/Engine/EditorBlueprintResources/StandardMacros.IsValid` (`self.AnimationRef`)
    (:`Is Valid`
      _)
    (:`Is Not Valid`
      (bind _asabp_fem_zombie (cast `/Game/Characters/Zombie/Animations/FemZombieAnimations/ABP_FemZombie` (`SkeletalMeshComponent.GetAnimInstance` (`self.Mesh`))))
      (bind _output_get (set `self.AnimationRef` _asabp_fem_zombie))))
  (if (`/Game/Characters/Zombie/Animations/FemZombieAnimations/ABP_FemZombie.bFemDamagingPlayer` _output_get)
    (`/Engine/EditorBlueprintResources/StandardMacros.IsValid` (`self.PlayerRef`)
      (:`Is Valid`
        _)
      (:`Is Not Valid`
        (bind _asbp_first_person_character (cast `/Game/FirstPerson/Blueprints/BP_FirstPersonCharacter` (`GameplayStatics.GetPlayerCharacter` 0)))
        (bind _output_get_2 (set `self.PlayerRef` _asbp_first_person_character))))
    (`AudioComponent.Play` (`self.AttackSound`) 0.0)
    (`/Game/FirstPerson/Blueprints/BP_FirstPersonCharacter.Take Damage` _output_get_2 (`self.EnemyDamage`))
    (set `/Game/Characters/Zombie/Animations/FemZombieAnimations/ABP_FemZombie.bFemDamagingPlayer` false _output_get)))

(fn `UserConstructionScript`)